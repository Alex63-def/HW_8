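; Player tank pawn Blueprint that connects the tank to its health widget and to the game's menus through UIHUD.
; BeginPlay passes the pawn to the health widget, and Tick turns that widget toward the camera using only X and Y, keeping it upright.
; When HealthComponent reaches zero health, Tick destroys the widget and shows the exit-game screen.
; The M key toggles the main menu through a FlipFlop.
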(event EventBeginPlay
  (bind _ashud_player_health (Utilities|Casting|CastToHUD_PlayerHealth (UserInterface|GetUserWidgetObject (Variables|Default|GetWidgetHealth))))
  (Variables|/Game/Widgets/HUD_PlayerHealth.HUD_PlayerHealth_C|SetBP_PlayerTank _ashud_player_health self))

(event Collision|EventActorBeginOverlap
  (params (OtherActor :type Actor%20Object%20Reference)))

(event EventTick
  (params (DeltaSeconds :type Float%20%28single-precision%29))
  (bind _self self)
  (bind _widgethealth (Variables|Default|GetWidgetHealth))
  (bind _returnvalue (Transformation|GetWorldLocation _widgethealth))
  (bind _camera (Variables|/Script/lesson_3.UnitPawn|GetCamera _self))
  (bind _returnvalue_2 (Transformation|GetWorldLocation _camera))
  (if (Utilities|IsValid (Variables|Default|GetWidgetHealth))
    (Transformation|SetWorldRotation _widgethealth (Math|Rotator|FindLookatRotation (Math|Vector|MakeVector (.x _returnvalue) (.y _returnvalue) 0.0) (Math|Vector|MakeVector (.x _returnvalue_2) (.y _returnvalue_2) 0.0)) false false)
    (if (== (Variables|/Script/lesson_3.HealthComponent|GetCurrentHealthTank (Variables|Default|GetHealthComponent)) 0.0)
      (Components|DestroyComponent (Variables|Default|GetWidgetHealth))
      (bind _asuihud (Utilities|Casting|CastToUIHUD (HUD|GetHUD (Game|GetPlayerController 0))))
      (Class|UIHUD|ShowWidget _asuihud "Wid_ExitGame"))))

(event Input|KeyboardEvents|M
  (params (Key :type Key%20Structure :default "None"))
  (:Pressed
    (bind _asuihud (Utilities|Casting|CastToUIHUD (HUD|GetHUD (Game|GetPlayerController 0))))
    (Utilities|FlowControl|FlipFlop
      (:A
        (Class|UIHUD|ShowWidget _asuihud "Wid_MainMenu"))
      (:B
        (Class|UIHUD|HideWidget _asuihud)))))

(fn ConstructionScript)