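; Enemy tank Blueprint that manages the floating health widget above an AI or enemy tank.
; BeginPlay hands itself to the HUD_EnemyTankHealth widget and caches the player's BP_TankPawn.
; Tick turns the widget toward the player's camera using only X and Y positions, then destroys it once HealthComponent reports zero health.
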(event EventBeginPlay
  (bind _ashud_enemy_tank_health (Utilities|Casting|CastToHUD_EnemyTankHealth (UserInterface|GetUserWidgetObject (Variables|Default|GetWidgetHealth))))
  (Variables|/Game/Widgets/HUD_EnemyTankHealth.HUD_EnemyTankHealth_C|SetBP_EnemyTank _ashud_enemy_tank_health self)
  (bind _asbp_tank_pawn (Utilities|Casting|CastToBP_TankPawn (Game|Player|GetPlayerPawn 0)))
  (Variables|Default|SetPlayer _asbp_tank_pawn))

(event Collision|EventActorBeginOverlap
  (params (OtherActor :type Actor%20Object%20Reference)))

(event EventTick
  (params (DeltaSeconds :type Float%20%28single-precision%29))
  (bind _widgethealth (Variables|Default|GetWidgetHealth))
  (bind _player (Variables|Default|GetPlayer))
  (bind _returnvalue (Transformation|GetWorldLocation _widgethealth))
  (bind _camera (Variables|/Script/lesson_3.UnitPawn|GetCamera _player))
  (bind _returnvalue_2 (Transformation|GetWorldLocation _camera))
  (if (Utilities|IsValid (Variables|Default|GetWidgetHealth))
    (Transformation|SetWorldRotation _widgethealth (Math|Rotator|FindLookatRotation (Math|Vector|MakeVector (.x _returnvalue) (.y _returnvalue) 0.0) (Math|Vector|MakeVector (.x _returnvalue_2) (.y _returnvalue_2) 0.0)) false false)
    (if (== (Variables|/Script/lesson_3.HealthComponent|GetCurrentHealthTank (Variables|Default|GetHealthComponent)) 0.0)
      (Components|DestroyComponent (Variables|Default|GetWidgetHealth)))))

(fn ConstructionScript)